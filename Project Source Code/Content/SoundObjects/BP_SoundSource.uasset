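; BP_SoundSource is a placeable sound emitter, with audio and Phonon source components, that plays mono WAV files loaded from disk at runtime.
; On BeginPlay it builds its settings widgets and registers web-server GET routes under its own name, both controlling file, playback, delay and volume.
; Delayed playback can add speed-of-sound travel time from distance to another actor.
; Helper functions rebuild attenuation overrides for spatialization settings.
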(event Custom|/VolumeMultiplier
  (params (Connection :type Connection%20Object%20Reference))
  ;[1 0 0.3984] Begin Play
  ;;[0.8984 1 0 1 100] Register API
  ;;;[0 0.2031 1 1 50] Set Volume Multiplier
  (CallFunction|APISetVolumeMultiplier Connection))

(event Custom|\APISetSoundWave
  (params (Connection :type Connection%20Object%20Reference))
  ;[1 0 0.3984] Begin Play
  ;;[0.8984 1 0 1 100] Register API
  ;;;[0.7813 0 1 1 50] SetSoundWave
  (CallFunction|/SetSoundWav Connection))

(event Custom|HideRotationControl
  ;[1 0.8906 0 1 50] Hide Rotation Transform
  (Widget|SetVisibility (Variables|/Game/UI/OrbitalMotionSettings.OrbitalMotionSettings_C|GetHBox_TransformRotation (Variables|Default|GetOrbital%20Motion%20Settings%20Widget self)) "Collapsed"))

(event Custom|UI%20Bind%20Sound%20Source%20Events
  ;[1 0.7969 0 1 100] UI Bind Sound Source Events
  (bind (_setwavfile _loadedsoundwavpath _playsoundbutton _volumespinbox) (Default|GetWaveVariables (Variables|Default|GetSound%20Source%20Audio%20Settings)))
  ;;[0 0.4375 1 1 50] Event Set SoundWav Clicked
  (EventDispatchers|BindEventtoOnClicked _setwavfile (delegate Custom|Set%20Wave%20Button%20Clicked))
  ;;[0.5 0 1 1 50] Event Play Audio Button
  (EventDispatchers|BindEventtoOnClicked _playsoundbutton (delegate Custom|Play%20Audio%20Button%20Clicked))
  ;;[0 0.3203 1 1 50] Event Delay From Spin Box Changed
  (EventDispatchers|AssignOnValueChanged (Variables|/Game/UI/SoundSourceWavSettings.SoundSourceWavSettings_C|GetDelaySpinBox (Variables|Default|GetSound%20Source%20Audio%20Settings)) (delegate Custom|OnValueChanged_Event_3))
  ;[1 0.07031 0] Volume Value Changed
  (EventDispatchers|AssignOnValueChanged _volumespinbox (delegate Custom|Volume%20Value%20Changed)))

(event Custom|Play%20With%20Speed%20Of%20Sound
  (params (Speed%20Of%20Sound :type Float%20%28single-precision%29) (Actor :type Actor%20Object%20Reference))
  (bind _audio (Variables|Default|GetAudio))
  (bind _delay_before_play (Variables|Default|GetDelay%20Before%20Play))
  ;[0.5469 0 1] Play With Speed Of Sound
  (if (Audio|Components|Audio|IsPlaying _audio)
    (Audio|Components|Audio|Stop _audio)
    (else
      (Utilities|IsValid Actor
        (:Is%20Valid
          (bind _sos_delay (CallFunction|SetSpeedOfSoundDelay Actor Speed%20Of%20Sound))
          (Utilities|FlowControl|RetriggerableDelay (+ _sos_delay _delay_before_play)))
        (:Is%20Not%20Valid
          (Utilities|FlowControl|RetriggerableDelay _delay_before_play)))
      (Audio|Components|Audio|Play (Variables|Default|GetAudio) 0.0))))

(event Custom|PlayAudio
  (bind _audio (Variables|Default|GetAudio))
  ;[1 0.1406 0] Play Audio
  (if (Audio|Components|Audio|IsPlaying _audio)
    (Audio|Components|Audio|Stop _audio)
    (else
      (Audio|Components|Audio|Play _audio 0.0))))

(event Custom|Play%20Delayed
  ;[1 0.1406 0] Play Audio
  (Utilities|FlowControl|RetriggerableDelay (Variables|Default|GetDelay%20Before%20Play))
  (Audio|Components|Audio|Play (Variables|Default|GetAudio) 0.0))

(event Custom|Play%20Audio%20Button%20Clicked
  ;[1 0.7969 0 1 100] UI Bind Sound Source Events
  ;;[0.5 0 1 1 50] Event Play Audio Button
  (CallFunction|PlayAudio self))

(event Custom|/PlaySound
  (params (Connection :type Connection%20Object%20Reference))
  ;[1 0 0.3984] Begin Play
  ;;[0.8984 1 0 1 100] Register API
  ;;;[0 0.2031 1 1 50] PlaySound
  (bind _returnvalue (Utilities|MTogglePlaySound)
    (:Exec
      (Class|Connection|SendResponse Connection (Class|Response|ConstructResponseExt _returnvalue)))))

(event Custom|Volume%20Value%20Changed
  (params (InValue :type Float%20%28single-precision%29))
  ;[1 0.07031 0] Volume Value Changed
  (Audio|Components|Audio|SetVolumeMultiplier (Variables|Default|GetAudio) InValue :!class /Script/Engine.AudioComponent))

(event Custom|/SoundWaveDetails
  (params (Connection :type Connection%20Object%20Reference))
  ;[1 0 0.3984] Begin Play
  ;;[0.8984 1 0 1 100] Register API
  ;;;[0 0.2031 1 1 50] Get Sound Wav Details
  (CallFunction|APIGetSoundWaveDetails Connection))

(event Custom|SetDelay
  (params (Connection :type Connection%20Object%20Reference))
  ;[1 0 0.3984] Begin Play
  ;;[0.8984 1 0 1 100] Register API
  ;;;[0 0.2031 1 1 50] Set Delay
  (CallFunction|APISetDelay Connection))

(event Custom|OnValueChanged_Event_3
  (params (InValue :type Float%20%28single-precision%29))
  ;[1 0.7969 0 1 100] UI Bind Sound Source Events
  ;;[0 0.3203 1 1 50] Event Delay From Spin Box Changed
  (Rendering|Components|TextRender|SetText (Variables|/Game/UI/SoundSourceWavSettings.SoundSourceWavSettings_C|GetDelayText (Variables|Default|GetSound%20Source%20Audio%20Settings)) (Utilities|Text|ToText(String) (Class|VictoryBPFunctionLibrary|VictorySecondstoHoursMinutesSeconds InValue true)))
  (Variables|Default|SetDelay%20Before%20Play InValue))

(event Custom|Set%20Selected%20Material
  ;[0 1 0.4844] Set Selected
  (Rendering|Material|SetMaterial (Variables|Default|GetStaticMesh) 0 "/Game/AutomotiveMaterials/Materials/Exterior/CarPaint/MI_CarPaint_LightBlue.MI_CarPaint_LightBlue"))

(event Custom|APISetSoundSettings
  (params (Connection :type Connection%20Object%20Reference))
  ;[1 0 0.9609] SetSettings
)

(event Custom|Set%20Regular%20Material
  ;[1 0 0.7266] Set Regular Material
  (Rendering|Material|SetMaterial (Variables|Default|GetStaticMesh) 0 "/Game/AutomotiveMaterials/Materials/Exterior/CarPaint/MI_CarPaint_DarkBlue.MI_CarPaint_DarkBlue"))

(event Custom|/GetSettings
  (params (Connection :type Connection%20Object%20Reference))
  ;[0.7812 1 0] Get Settings
)

(event Custom|Set%20Wave%20Button%20Clicked
  ;[1 0.7969 0 1 100] UI Bind Sound Source Events
  ;;[0 0.4375 1 1 50] Event Set SoundWav Clicked
  (bind (_outfilenames _returnvalue) (Class|EFDFunctionLibrary|OpenFileDialog "Select MONO wav file" (Variables|/Game/Controller/BP_PlayerController.BP_PlayerController_C|GetLast%20Wav%20file%20path (Utilities|GetController)) "" "*.wav" "Single"))
  (if _returnvalue
    (CallFunction|UISetSoundWav (Utilities|Array|Get(acopy) _outfilenames))))

(event Custom|Load%20Sound%20Wav
  (params (path :type String))
  ;[0.3594 0 1 1 100] Load Wav File
  ;;[0 0.9297 1 1 50] Stop Sound If Playing
  (if (Audio|Components|Audio|IsPlaying (Variables|Default|GetAudio))
    (Audio|Components|Audio|Stop (Variables|Default|GetAudio)))
  (bind _output_get (Variables|Default|SetSet%20Wav%20Op%20Success (Class|BlueprintPathsLibrary|FileExists path)))
  (if _output_get
    (bind _output_get_2 (Variables|Default|SetSound%20Wav%20Path path))
    (bind (_success _returnvalue) (Class|AudioFunctions|GetSoundfromWaveFile _output_get_2))
    (bind _output_get_3 (Variables|Default|SetSet%20Wav%20Op%20Success _success))
    (Utilities|IsValid _returnvalue
      (:Is%20Valid
        (if _output_get_3
          (bind _output_get_4 (Variables|Default|SetSound%20Wav _returnvalue))
          (Variables|Default|SetWav%20Duration (Variables|/Script/Engine.SoundBase|GetDuration _output_get_4))
          (Audio|Components|Audio|SetSound (Variables|Default|GetAudio) _output_get_4)
          (Variables|Default|SetSet%20Wav%20Op%20Details (Utilities|String|Append "Sound Source " (Variables|Default|GetName self) ": " (Class|BlueprintPathsLibrary|GetCleanFilename (Variables|Default|GetSound%20Wav%20Path)) " was set as WAV file"))
          (else
            (bind _output_get_5 (Variables|Default|SetSet%20Wav%20Op%20Details (Utilities|String|Append "ERROR: Failed to read wav file from " (Variables|Default|GetSound%20Wav%20Path)) :!label _label))
            (Development|PrintString _output_get_5))))
      (:Is%20Not%20Valid
        (Development|PrintString "ERROR: Invalid File - WAV must be mono")
        (goto _label)))
    (Development|PrintString (Variables|Default|GetSet%20Wav%20Op%20Details))
    (else
      (bind _output_get_6 (Variables|Default|SetSet%20Wav%20Op%20Details (Utilities|String|Append "ERROR: Path `" "" "` does not exist")))
      (Development|PrintString _output_get_6))))

(event EventEndPlay
  (params (EndPlayReason :type EEndPlayReason%20Enum :default "Destroyed"))
  (bind _audio (Variables|Default|GetAudio))
  ;[1 0 0.09375] End Play
  (if (Audio|Components|Audio|IsPlaying _audio)
    (Audio|Components|Audio|StopDelayed _audio 0.0)
    (Components|DestroyComponent _audio)))

(event EventBeginPlay
  (bind _output (Utilities|MGetWebServer))
  (bind _output_2 (Utilities|GetController))
  ;[1 0 0.3984] Begin Play
  (|CallParentFunction)
  ;;[1 0.6563 0 1 50] Hide Rotation
  (CallFunction|HideRotationControl)
  ;;[0.8281 0 1 1 50] Create Sound Source Settings Widget
  (bind _returnvalue (UserInterface|CreateWidget "/Game/UI/SoundObjectSettings.SoundObjectSettings_C" _output_2))
  (Variables|Default|SetSoundSource%20Settings%20Widget _returnvalue)
  ;;[1 0 0.09375 1 50] Create Audio Settings Widget and Init
  (bind _returnvalue_2 (UserInterface|CreateWidget "/Game/UI/SoundSourceWavSettings.SoundSourceWavSettings_C" _output_2))
  (bind _output_get (Variables|Default|SetSound%20Source%20Audio%20Settings _returnvalue_2))
  (Class|SpinBox|SetMinSliderValue (Variables|/Game/UI/SoundSourceWavSettings.SoundSourceWavSettings_C|GetDelaySpinBox _output_get) 0.0)
  (Class|SpinBox|SetMinValue (Variables|/Game/UI/SoundSourceWavSettings.SoundSourceWavSettings_C|GetDelaySpinBox _output_get) 0.0)
  ;;[0.1953 1 0 1 50] Populate Settings Widget
  (Class|VerticalBox|AddChildtoVerticalBox (Variables|/Game/UI/SoundObjectSettings.SoundObjectSettings_C|GetVBOX (Variables|Default|GetSoundSource%20Settings%20Widget)) (Variables|Default|GetOrbital%20Motion%20Settings%20Widget self))
  (Class|VerticalBox|AddChildtoVerticalBox (Variables|/Game/UI/SoundObjectSettings.SoundObjectSettings_C|GetVBOX (Variables|Default|GetSoundSource%20Settings%20Widget)) _output_get)
  ;;[0.5234 0 1 1 50] Bind UI Events
  (CallFunction|UIBindSoundSourceEvents)
  ;;[0.8984 1 0 1 100] Register API
  ;;;[0.7813 0 1 1 50] SetSoundWave
  (Class|WebServer|AddURIHandler _output (Utilities|String|Append "/" (Variables|Default|GetName) "/SetSoundWave") (delegate Custom|\APISetSoundWave) "VE_GET" true)
  ;;;[0 0.2031 1 1 50] PlaySound
  (Class|WebServer|AddURIHandler _output (Utilities|String|Append "/" (Variables|Default|GetName) "/PlaySound") (delegate Custom|/PlaySound) "VE_GET" true)
  ;;;[0 0.2031 1 1 50] Set Delay
  (Class|WebServer|AddURIHandler _output (Utilities|String|Append "/" (Variables|Default|GetName) "/SetDelay") (delegate Custom|SetDelay) "VE_GET" true)
  ;;;[0 0.2031 1 1 50] Get Sound Wav Details
  (Class|WebServer|AddURIHandler _output (Utilities|String|Append "/" (Variables|Default|GetName) "/SoundWaveDetails") (delegate Custom|/SoundWaveDetails) "VE_GET" true)
  ;;;[0 0.2031 1 1 50] Set Volume Multiplier
  (Class|WebServer|AddURIHandler _output (Utilities|String|Append "/" (Variables|Default|GetName) "/VolumeMultiplier") (delegate Custom|/VolumeMultiplier) "VE_GET" true))

(event Custom|/GetSoundSettings
  (params (connection :type Connection%20Object%20Reference))
  (bind _returnvalue (Class|HeadMountedDisplayFunctionLibrary|GetWorldtoMetersScale))
  (bind _audio (Variables|Default|GetAudio))
  (bind _attenuationoverrides (Variables|/Script/Engine.AudioComponent|GetAttenuationOverrides _audio))
  (bind (_battenuate _bspatialize _bapplynormalizationtostereosounds _spatializationalgorithm _binauralradius _omniradius _stereospread _distancealgorithm _dbattenuationatmax _attenuationshapeextents _falloffdistance) (Utilities|Struct|BreakSoundAttenuationSettings _attenuationoverrides))
  (bind _returnvalue_2 (Class|BlueprintJsonLibrary|JsonSetField (Class|BlueprintJsonLibrary|JsonMake) (Utilities|String|MakeLiteralString "enable_volume_attenuation") (Class|BlueprintJsonLibrary|JsonMakeBool _battenuate)))
  (bind _returnvalue_3 (Class|BlueprintJsonLibrary|JsonSetField _returnvalue_2 (Utilities|String|MakeLiteralString "enable_spatialization") (Class|BlueprintJsonLibrary|JsonMakeBool _bspatialize)))
  (bind _returnvalue_4 (Class|BlueprintJsonLibrary|JsonSetField _returnvalue_3 (Utilities|String|MakeLiteralString "normalize_3d_stereo_sounds") (Class|BlueprintJsonLibrary|JsonMakeBool _bapplynormalizationtostereosounds)))
  (bind _returnvalue_5 (Class|BlueprintJsonLibrary|JsonSetField _returnvalue_4 (Utilities|String|MakeLiteralString "spatialization_method") (Class|BlueprintJsonLibrary|JsonMakeString (Utilities|String|EnumtoString _spatializationalgorithm))))
  (bind _returnvalue_6 (Class|BlueprintJsonLibrary|JsonSetField _returnvalue_5 (Utilities|String|MakeLiteralString "binaural_radius") (Class|BlueprintJsonLibrary|JsonMakeFloat (/ _binauralradius _returnvalue))))
  (bind _returnvalue_7 (Class|BlueprintJsonLibrary|JsonSetField _returnvalue_6 (Utilities|String|MakeLiteralString "non_spatialized_radius") (Class|BlueprintJsonLibrary|JsonMakeFloat (/ _returnvalue _omniradius))))
  (bind _returnvalue_8 (Class|BlueprintJsonLibrary|JsonSetField _returnvalue_7 (Utilities|String|MakeLiteralString "3d_stereo_spread") (Class|BlueprintJsonLibrary|JsonMakeFloat _stereospread)))
  (bind _returnvalue_9 (Class|BlueprintJsonLibrary|JsonSetField _returnvalue_8 (Utilities|String|MakeLiteralString "attenuation_function") (Class|BlueprintJsonLibrary|JsonMakeString (Utilities|String|EnumtoString _distancealgorithm))))
  (bind _returnvalue_10 (Class|BlueprintJsonLibrary|JsonSetField _returnvalue_9 (Utilities|String|MakeLiteralString "attenuation_at_max") (Class|BlueprintJsonLibrary|JsonMakeFloat _dbattenuationatmax)))
  (bind _returnvalue_11 (Class|BlueprintJsonLibrary|JsonSetField _returnvalue_10 (Utilities|String|MakeLiteralString "inner_radius") (Class|BlueprintJsonLibrary|JsonMakeFloat (/ _returnvalue (.X (Math|Vector|BreakVector _attenuationshapeextents))))))
  (bind _returnvalue_12 (Class|BlueprintJsonLibrary|JsonSetField _returnvalue_11 (Utilities|String|MakeLiteralString "falloff_distance") (Class|BlueprintJsonLibrary|JsonMakeFloat (/ _returnvalue _falloffdistance))))
  (Class|Connection|SendResponse connection (Class|Response|ConstructResponseExt (Class|BlueprintJsonLibrary|ToPrettyString(JsonObject) _returnvalue_12))))

(fn ConstructionScript
  (Rendering|Components|TextRender|SetText (Variables|Default|GetTextRender) (Utilities|Text|ToText(String) (Variables|Default|GetName))))

(fn SetSoundWave
  (params (Path :type String)))

(fn APISetSoundWave
  (params (connection :type Connection%20Object%20Reference)))

(fn PlaySound
  (bind _audio (Variables|Default|GetAudio))
  (if (Audio|Components|Audio|IsPlaying _audio)
    (Audio|Components|Audio|Stop _audio)
    (else
      (Audio|Components|Audio|Play _audio 0.0))))

(fn GetSpeaker)

(fn ForTest
  (Development|PrintString (Utilities|String|EnumtoString (.SpatializationAlgorithm (Utilities|Struct|BreakSoundAttenuationSettings (Variables|/Script/Engine.AudioComponent|GetAttenuationOverrides (Variables|Default|GetAudio)))))))

(fn /SetSoundWav
  (params (Connection :type Connection%20Object%20Reference))
  (bind _output (Utilities|GetController))
  (bind (_set_wav_op_success _set_wav_op_details) (CallFunction|UISetSoundWav (Class|Connection|GetGETVar Connection "path")))
  (bind _json (Default|(Success,Details)->json _output _set_wav_op_success _set_wav_op_details))
  (Default|Json->response->send _output Connection _json))

(fn SetSoundWav
  (params (filePath :type String))
  (bind _output_get (LocalVariables|SetSuccess (Class|BlueprintPathsLibrary|FileExists filePath)))
  (if _output_get
    (bind _output_get_2 (Variables|Default|SetSound%20Wav%20Path filePath))
    (bind (_success _returnvalue) (Class|AudioFunctions|GetSoundfromWaveFile _output_get_2))
    (bind _output_get_3 (LocalVariables|SetSuccess _success))
    (if _output_get_3
      (bind _output_get_4 (Variables|Default|SetSound%20Wav _returnvalue))
      (Variables|Default|SetWav%20Duration (Variables|/Script/Engine.SoundBase|GetDuration _output_get_4))
      (if (Audio|Components|Audio|IsPlaying (Variables|Default|GetAudio))
        (Audio|Components|Audio|Stop (Variables|Default|GetAudio))
        (Audio|Components|Audio|SetSound (Variables|Default|GetAudio) _output_get_4)
        (LocalVariables|SetDetails (Utilities|String|Append "Sound Source " "" " " (Variables|Default|GetSound%20Wav%20Path) " was set as WAV file"))
        ;[0 1 0.3672] Return
        (return (LocalVariables|GetDetails) (LocalVariables|GetSuccess)))
      (else
        (LocalVariables|SetDetails (Utilities|String|Append "ERROR: Failed to read wav file from " (Variables|Default|GetSound%20Wav%20Path)))
        (return (LocalVariables|GetDetails) (LocalVariables|GetSuccess))))
    (else
      (LocalVariables|SetDetails (Utilities|String|Append "ERROR: Path `" filePath "` does not exist"))
      (return (LocalVariables|GetDetails) (LocalVariables|GetSuccess)))))

(fn ChangeSoundSettings
  (params (Change%20Enable%20Spatialization :type Boolean) (Enable%20Spatialization :type Boolean) (Change%20Method :type Boolean) (Spatialization%20method :type String) (Change%20Binaural%20Radius :type Boolean) (Binaural%20Radius :type Float%20%28single-precision%29) (Change%20NS%20Radius :type Boolean) (Non%20-%20Spatialized%20Radius :type Float%20%28single-precision%29) (Change%203D%20Stereo%20Spread :type Boolean) (3D%20Stereo%20Spread :type Float%20%28single-precision%29) (Normalize%203D%20Sounds :type Boolean) (Change%20Normalize%203D%20Sounds :type Boolean))
  (if Change%20Enable%20Spatialization
    (Variables|/Script/Engine.AudioComponent|SetbAllowSpatialization (Variables|Default|GetAudio) Enable%20Spatialization))
  (if Change%20Method
    (Development|PrintString "Switch")
    (switch string Spatialization%20method
      (:Binaural
        (LocalVariables|SetLocal%20Spatialization%20Method "SPATIALIZATION_HRTF"))
      (:Panning
        (LocalVariables|SetLocal%20Spatialization%20Method "SPATIALIZATION_Default"))))
  (bind _output_get (Variables|Default|SetSource%20Attenuation%20Settings (Utilities|Struct|MakeSoundAttenuationSettings (.bAttenuate (Utilities|Struct|BreakSoundAttenuationSettings (Variables|Default|GetSource%20Attenuation%20Settings))) (.bSpatialize (Utilities|Struct|BreakSoundAttenuationSettings (Variables|Default|GetSource%20Attenuation%20Settings))) (.bAttenuateWithLPF (Utilities|Struct|BreakSoundAttenuationSettings (Variables|Default|GetSource%20Attenuation%20Settings))) (.bEnableListenerFocus (Utilities|Struct|BreakSoundAttenuationSettings (Variables|Default|GetSource%20Attenuation%20Settings))) (.bEnableFocusInterpolation (Utilities|Struct|BreakSoundAttenuationSettings (Variables|Default|GetSource%20Attenuation%20Settings))) (.bEnableOcclusion (Utilities|Struct|BreakSoundAttenuationSettings (Variables|Default|GetSource%20Attenuation%20Settings))) (.bUseComplexCollisionForOcclusion (Utilities|Struct|BreakSoundAttenuationSettings (Variables|Default|GetSource%20Attenuation%20Settings))) (.bEnableReverbSend (Utilities|Struct|BreakSoundAttenuationSettings (Variables|Default|GetSource%20Attenuation%20Settings))) (.bEnablePriorityAttenuation (Utilities|Struct|BreakSoundAttenuationSettings (Variables|Default|GetSource%20Attenuation%20Settings))) (select Change%20Normalize%203D%20Sounds Normalize%203D%20Sounds (.bApplyNormalizationToStereoSounds (Utilities|Struct|BreakSoundAttenuationSettings (Variables|Default|GetSource%20Attenuation%20Settings)))) (.bEnableLogFrequencyScaling (Utilities|Struct|BreakSoundAttenuationSettings (Variables|Default|GetSource%20Attenuation%20Settings))) (.bEnableSubmixSends (Utilities|Struct|BreakSoundAttenuationSettings (Variables|Default|GetSource%20Attenuation%20Settings))) (select Change%20Method (LocalVariables|GetLocal%20Spatialization%20Method) (.SpatializationAlgorithm (Utilities|Struct|BreakSoundAttenuationSettings (Variables|Default|GetSource%20Attenuation%20Settings)))) (Math|Float|SelectFloat Binaural%20Radius (.BinauralRadius (Utilities|Struct|BreakSoundAttenuationSettings (Variables|Default|GetSource%20Attenuation%20Settings))) Change%20Binaural%20Radius) (.AbsorptionMethod (Utilities|Struct|BreakSoundAttenuationSettings (Variables|Default|GetSource%20Attenuation%20Settings))) (.OcclusionTraceChannel (Utilities|Struct|BreakSoundAttenuationSettings (Variables|Default|GetSource%20Attenuation%20Settings))) (.ReverbSendMethod (Utilities|Struct|BreakSoundAttenuationSettings (Variables|Default|GetSource%20Attenuation%20Settings))) (.PriorityAttenuationMethod (Utilities|Struct|BreakSoundAttenuationSettings (Variables|Default|GetSource%20Attenuation%20Settings))) (Math|Float|SelectFloat Non%20-%20Spatialized%20Radius (.OmniRadius (Utilities|Struct|BreakSoundAttenuationSettings (Variables|Default|GetSource%20Attenuation%20Settings))) Change%20NS%20Radius) (Math|Float|SelectFloat 3D%20Stereo%20Spread (.StereoSpread (Utilities|Struct|BreakSoundAttenuationSettings (Variables|Default|GetSource%20Attenuation%20Settings))) Change%203D%20Stereo%20Spread) (.LPFRadiusMin (Utilities|Struct|BreakSoundAttenuationSettings (Variables|Default|GetSource%20Attenuation%20Settings))) (.LPFRadiusMax (Utilities|Struct|BreakSoundAttenuationSettings (Variables|Default|GetSource%20Attenuation%20Settings))) (.CustomLowpassAirAbsorptionCurve (Utilities|Struct|BreakSoundAttenuationSettings (Variables|Default|GetSource%20Attenuation%20Settings))) (.CustomHighpassAirAbsorptionCurve (Utilities|Struct|BreakSoundAttenuationSettings (Variables|Default|GetSource%20Attenuation%20Settings))) (.LPFFrequencyAtMin (Utilities|Struct|BreakSoundAttenuationSettings (Variables|Default|GetSource%20Attenuation%20Settings))) (.LPFFrequencyAtMax (Utilities|Struct|BreakSoundAttenuationSettings (Variables|Default|GetSource%20Attenuation%20Settings))) (.HPFFrequencyAtMin (Utilities|Struct|BreakSoundAttenuationSettings (Variables|Default|GetSource%20Attenuation%20Settings))) (.HPFFrequencyAtMax (Utilities|Struct|BreakSoundAttenuationSettings (Variables|Default|GetSource%20Attenuation%20Settings))) (.FocusAzimuth (Utilities|Struct|BreakSoundAttenuationSettings (Variables|Default|GetSource%20Attenuation%20Settings))) (.NonFocusAzimuth (Utilities|Struct|BreakSoundAttenuationSettings (Variables|Default|GetSource%20Attenuation%20Settings))) (.FocusDistanceScale (Utilities|Struct|BreakSoundAttenuationSettings (Variables|Default|GetSource%20Attenuation%20Settings))) (.NonFocusDistanceScale (Utilities|Struct|BreakSoundAttenuationSettings (Variables|Default|GetSource%20Attenuation%20Settings))) (.FocusPriorityScale (Utilities|Struct|BreakSoundAttenuationSettings (Variables|Default|GetSource%20Attenuation%20Settings))) (.NonFocusPriorityScale (Utilities|Struct|BreakSoundAttenuationSettings (Variables|Default|GetSource%20Attenuation%20Settings))) (.FocusVolumeAttenuation (Utilities|Struct|BreakSoundAttenuationSettings (Variables|Default|GetSource%20Attenuation%20Settings))) (.NonFocusVolumeAttenuation (Utilities|Struct|BreakSoundAttenuationSettings (Variables|Default|GetSource%20Attenuation%20Settings))) (.FocusAttackInterpSpeed (Utilities|Struct|BreakSoundAttenuationSettings (Variables|Default|GetSource%20Attenuation%20Settings))) (.FocusReleaseInterpSpeed (Utilities|Struct|BreakSoundAttenuationSettings (Variables|Default|GetSource%20Attenuation%20Settings))) (.OcclusionLowPassFilterFrequency (Utilities|Struct|BreakSoundAttenuationSettings (Variables|Default|GetSource%20Attenuation%20Settings))) (.OcclusionVolumeAttenuation (Utilities|Struct|BreakSoundAttenuationSettings (Variables|Default|GetSource%20Attenuation%20Settings))) (.OcclusionInterpolationTime (Utilities|Struct|BreakSoundAttenuationSettings (Variables|Default|GetSource%20Attenuation%20Settings))) (.ReverbWetLevelMin (Utilities|Struct|BreakSoundAttenuationSettings (Variables|Default|GetSource%20Attenuation%20Settings))) (.ReverbWetLevelMax (Utilities|Struct|BreakSoundAttenuationSettings (Variables|Default|GetSource%20Attenuation%20Settings))) (.ReverbDistanceMin (Utilities|Struct|BreakSoundAttenuationSettings (Variables|Default|GetSource%20Attenuation%20Settings))) (.ReverbDistanceMax (Utilities|Struct|BreakSoundAttenuationSettings (Variables|Default|GetSource%20Attenuation%20Settings))) (.ManualReverbSendLevel (Utilities|Struct|BreakSoundAttenuationSettings (Variables|Default|GetSource%20Attenuation%20Settings))) (.CustomReverbSendCurve (Utilities|Struct|BreakSoundAttenuationSettings (Variables|Default|GetSource%20Attenuation%20Settings))) (.SubmixSendSettings (Utilities|Struct|BreakSoundAttenuationSettings (Variables|Default|GetSource%20Attenuation%20Settings))) (.PriorityAttenuationMin (Utilities|Struct|BreakSoundAttenuationSettings (Variables|Default|GetSource%20Attenuation%20Settings))) (.PriorityAttenuationMax (Utilities|Struct|BreakSoundAttenuationSettings (Variables|Default|GetSource%20Attenuation%20Settings))) (.PriorityAttenuationDistanceMin (Utilities|Struct|BreakSoundAttenuationSettings (Variables|Default|GetSource%20Attenuation%20Settings))) (.PriorityAttenuationDistanceMax (Utilities|Struct|BreakSoundAttenuationSettings (Variables|Default|GetSource%20Attenuation%20Settings))) (.ManualPriorityAttenuation (Utilities|Struct|BreakSoundAttenuationSettings (Variables|Default|GetSource%20Attenuation%20Settings))) (.CustomPriorityAttenuationCurve (Utilities|Struct|BreakSoundAttenuationSettings (Variables|Default|GetSource%20Attenuation%20Settings))) (.PluginSettings (Utilities|Struct|BreakSoundAttenuationSettings (Variables|Default|GetSource%20Attenuation%20Settings))) (.DistanceAlgorithm (Utilities|Struct|BreakSoundAttenuationSettings (Variables|Default|GetSource%20Attenuation%20Settings))) (.AttenuationShape (Utilities|Struct|BreakSoundAttenuationSettings (Variables|Default|GetSource%20Attenuation%20Settings))) (.dBAttenuationAtMax (Utilities|Struct|BreakSoundAttenuationSettings (Variables|Default|GetSource%20Attenuation%20Settings))) (.FalloffMode (Utilities|Struct|BreakSoundAttenuationSettings (Variables|Default|GetSource%20Attenuation%20Settings))) (.AttenuationShapeExtents (Utilities|Struct|BreakSoundAttenuationSettings (Variables|Default|GetSource%20Attenuation%20Settings))) (.ConeOffset (Utilities|Struct|BreakSoundAttenuationSettings (Variables|Default|GetSource%20Attenuation%20Settings))) (.FalloffDistance (Utilities|Struct|BreakSoundAttenuationSettings (Variables|Default|GetSource%20Attenuation%20Settings))) (.CustomAttenuationCurve (Utilities|Struct|BreakSoundAttenuationSettings (Variables|Default|GetSource%20Attenuation%20Settings))))))
  (Variables|/Script/Engine.AudioComponent|SetAttenuationOverrides (Variables|Default|GetAudio) _output_get))

(fn UISetSoundWav
  (params (Filename :type String))
  (bind _returnvalue (Class|KismetSystemLibrary|ConverttoAbsolutePath Filename))
  (bind _sound_source_audio_settings (Variables|Default|GetSound%20Source%20Audio%20Settings))
  (bind _set_wav_op_success (Variables|Default|GetSet%20Wav%20Op%20Success))
  (bind _loadedsoundwavpath (Variables|/Game/UI/SoundSourceWavSettings.SoundSourceWavSettings_C|GetLoadedSoundWavPath _sound_source_audio_settings))
  (bind _playsoundbutton (Variables|/Game/UI/SoundSourceWavSettings.SoundSourceWavSettings_C|GetPlaySoundButton _sound_source_audio_settings))
  (CallFunction|LoadSoundWav _returnvalue)
  (Variables|/Game/Controller/BP_PlayerController.BP_PlayerController_C|SetLast%20Wav%20file%20path (Utilities|GetController) (Utilities|Paths|GetPath _returnvalue))
  (if _set_wav_op_success
    (Widget|SetIsEnabled _playsoundbutton true)
    (Rendering|Components|TextRender|SetText _loadedsoundwavpath (Utilities|Text|ToText(String) _returnvalue))
    (else
      (Widget|SetIsEnabled _playsoundbutton false)
      (Rendering|Components|TextRender|SetText _loadedsoundwavpath "")))
  (return _set_wav_op_success (Variables|Default|GetSet%20Wav%20Op%20Details)))

(fn APISetDelay
  (params (Connection :type Connection%20Object%20Reference))
  (bind _returnvalue (Class|Connection|GetGETVar Connection "delay"))
  (bind _self self)
  (bind _sound_source_audio_settings (Variables|Default|GetSound%20Source%20Audio%20Settings))
  (bind _returnvalue_2 (Math|Conversions|ToFloat(Integer) _returnvalue))
  (bind _returnvalue_3 (Class|VictoryBPFunctionLibrary|VictorySecondstoHoursMinutesSeconds _returnvalue_2 true))
  (bind _output_get (LocalVariables|SetLocal%20Success (>= _returnvalue_2 0.0)))
  (if _output_get
    (Class|SpinBox|SetValue (Variables|/Game/UI/SoundSourceWavSettings.SoundSourceWavSettings_C|GetDelaySpinBox _sound_source_audio_settings) _returnvalue_2)
    (Rendering|Components|TextRender|SetText (Variables|/Game/UI/SoundSourceWavSettings.SoundSourceWavSettings_C|GetDelayText _sound_source_audio_settings) (Utilities|Text|ToText(String) _returnvalue_3))
    (LocalVariables|SetLocal%20Details (Utilities|String|Append (Variables|Default|GetName self) ": " " Delay set to " _returnvalue_3))
    (else
      (LocalVariables|SetLocal%20Details "Error: Delay value must be non-negative")))
  (bind _json (Default|(Success,Details)->json _self (LocalVariables|GetLocal%20Success) (LocalVariables|GetLocal%20Details)))
  (Default|Json->response->send _self _json Connection)
  (return (LocalVariables|GetLocal%20Details) (LocalVariables|GetLocal%20Success)))

(fn APIGetSoundWaveDetails
  (params (Connection :type Connection%20Object%20Reference))
  (bind _sound_wav_path (Variables|Default|GetSound%20Wav%20Path))
  (Variables|Default|GetSound%20Wav
    (:then
      (LocalVariables|SetLocal%20Success true))
    (:else
      (LocalVariables|SetLocal%20Success false)))
  (if (LocalVariables|GetLocal%20Success)
    (bind _returnvalue (Class|BlueprintJsonLibrary|JsonSetField (Class|BlueprintJsonLibrary|JsonMake) "file name" (Class|BlueprintJsonLibrary|JsonMakeString (Class|BlueprintPathsLibrary|GetCleanFilename _sound_wav_path))))
    (bind _returnvalue_2 (Class|BlueprintJsonLibrary|JsonSetField _returnvalue "path" (Class|BlueprintJsonLibrary|JsonMakeString (Utilities|Paths|GetPath _sound_wav_path))))
    (bind _returnvalue_3 (Class|BlueprintJsonLibrary|JsonSetField _returnvalue_2 "delay" (Class|BlueprintJsonLibrary|JsonMakeFloat (Variables|Default|GetDelay%20Before%20Play))))
    (Default|Json->response->send self _returnvalue_3 Connection)
    (else
      (bind _output_get (LocalVariables|SetLocal%20Details (Utilities|String|Append "Error: " (Variables|Default|GetName self) " has no sound wave associated with it")))
      (bind _json (Default|(Success,Details)->json self (LocalVariables|GetLocal%20Success) _output_get))
      (CallFunction|Json->response->send _json Connection)))
  (return (LocalVariables|GetLocal%20Details) (LocalVariables|GetLocal%20Success)))

(fn APISetVolumeMultiplier
  (params (Connection :type Connection%20Object%20Reference))
  (bind _returnvalue (Class|Connection|GetGETVar Connection "multiplier"))
  (bind _returnvalue_2 (Math|Conversions|ToFloat(Integer) _returnvalue))
  (bind _output_get (LocalVariables|SetSuccess (Math|Float|InRange(Float) _returnvalue_2 0.01 2.0)))
  (if _output_get
    (LocalVariables|SetDetails (Class|VictoryBPFunctionLibrary|AppendMultiple (Class|KismetSystemLibrary|GetPathName self) ": Volume multiplier set to " (Utilities|String|ToString(Float) _returnvalue_2)))
    (Class|SpinBox|SetValue (Variables|/Game/UI/SoundSourceWavSettings.SoundSourceWavSettings_C|GetVolumeSpinBox (Variables|Default|GetSound%20Source%20Audio%20Settings)) _returnvalue_2)
    (else
      (LocalVariables|SetDetails "Error: Volume allowed in range [0.01,2.0]")))
  (bind _json (CallFunction|(Success,Details)->json (LocalVariables|GetSuccess) (LocalVariables|GetDetails)))
  (CallFunction|Json->response->send _json Connection))

(fn SetSpeedOfSoundDelay
  (params (OtherActor :type Actor%20Object%20Reference) (Speed%20Of%20Sound :type Float%20%28single-precision%29))
  (bind _output_get (Variables|Default|SetSOS%20Delay (/ (/ (Transformation|GetDistanceTo OtherActor) (Class|HeadMountedDisplayFunctionLibrary|GetWorldtoMetersScale)) Speed%20Of%20Sound)))
  (return _output_get))

(fn GetEstimatedPlayTime
  (params (OtherActor :type Actor%20Object%20Reference) (Speed%20Of%20Sound :type Float%20%28single-precision%29))
  (bind _sos_delay (Variables|Default|GetSOS%20Delay))
  (if (!= _sos_delay 0.0)
    (return (+ (Variables|Default|GetDelay%20Before%20Play) (Variables|Default|GetWav%20Duration) _sos_delay))
    (else
      (return -1.0))))