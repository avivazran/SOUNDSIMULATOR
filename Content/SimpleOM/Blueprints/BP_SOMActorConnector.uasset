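; BP_SOMActorConnector is a connector actor that links the world positions of two referenced actors.
; A shared UpdatePositions function first moves the connector to FollowActor's location, then moves AttachActor to the connector's location, skipping any invalid reference.
; It runs from the construction script and every Tick, copying location only, without sweep or true component attachment.
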(event EventBeginPlay)

(event Collision|EventActorBeginOverlap
  (params (OtherActor :type Actor%20Object%20Reference)))

(event EventTick
  (params (DeltaSeconds :type Float%20%28single-precision%29))
  (CallFunction|UpdatePositions))

(fn ConstructionScript
  (CallFunction|UpdatePositions))

(fn UpdatePositions
  (bind _follow_actor (Variables|Default|GetFollow%20Actor))
  (bind _attach_actor (Variables|Default|GetAttach%20Actor))
  (Utilities|FlowControl|Sequence
    (:then_0
      (Utilities|IsValid _follow_actor
        (:Is%20Valid
          (Transformation|SetActorLocation (Transformation|GetActorLocation _follow_actor) false false))))
    (:then_1
      (Utilities|IsValid _attach_actor
        (:Is%20Valid
          (Transformation|SetActorLocation _attach_actor (Transformation|GetActorLocation) false false))))))