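; Actor that spawns a seeded, randomized set of child actors of a chosen class and moves them along orbits.
; InitiateActors, run in construction and at BeginPlay, generates orbit data from the seed and rebuilds one child actor component per orbit.
; While enabled, Tick recomputes each transform from time since creation using CalculateObjectTransform.
; Optional debug drawing shows orbits as instanced plane meshes in editor or play.
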(event EventBeginPlay
  (|CallParentFunction)
  (CallFunction|InitiateActors)
  (if (Variables|Default|GetEnable%20Debug%20Orbits)
    (CallFunction|DrawDebugOrbits)))

(event Collision|EventActorBeginOverlap
  (params (OtherActor :type Actor%20Object%20Reference))
  (|CallParentFunction OtherActor) ; This node is disabled and will not be called.\nDrag off pins to build functionality.
)

(event EventTick
  (params (DeltaSeconds :type Float%20%28single-precision%29))
  (|CallParentFunction DeltaSeconds)
  (if (Variables|Default|GetEnable%20SOM)
    (CallFunction|UpdateAllActors (Actor|GetGameTimeSinceCreation))))

(fn ConstructionScript
  (|CallParentFunction)
  (CallFunction|InitiateActors)
  (if (Variables|Default|GetShow%20Debug%20Orbits%20in%20Editor)
    (CallFunction|DrawDebugOrbits)))

(fn UpdateAllActors
  (params (New%20Time :type Float%20%28single-precision%29))
  (for (_array_element _array_index) (Variables|Default|GetOrbit%20Data)
    (bind (_new_location _new_rotation) (CallFunction|CalculateObjectTransform (.OrbitOffset (Utilities|Struct|BreakStruct_SOMData _array_element)) (.OrbitRotation (Utilities|Struct|BreakStruct_SOMData _array_element)) (.OrbitRadius (Utilities|Struct|BreakStruct_SOMData _array_element)) (.StartAngle (Utilities|Struct|BreakStruct_SOMData _array_element)) (.MovementSpeed (Utilities|Struct|BreakStruct_SOMData _array_element)) (.RotationSpeed (Utilities|Struct|BreakStruct_SOMData _array_element)) (.DefaultRotation (Utilities|Struct|BreakStruct_SOMData _array_element)) (.RotaterelativetoOrbit (Utilities|Struct|BreakStruct_SOMData _array_element)) New%20Time))
    (Transformation|SetWorldTransform (Utilities|Array|Get(acopy) (Variables|Default|GetActorArray) _array_index) (Math|Transform|MakeTransform _new_location _new_rotation (.DefaultScale (Utilities|Struct|BreakStruct_SOMData _array_element))) false false)))

(fn InitiateActors
  (bind _output_get (Variables|Default|SetGeneration%20Stream (Math|Random|MakeRandomStream (Variables|SpawnSettings|GetSeed))))
  (Class|KismetMathLibrary|ResetRandomStream _output_get)
  (Utilities|Array|Clear (Variables|Default|GetOrbit%20Data))
  (bind _data (CallFunction|GenerateRandomData (Variables|Default|GetGeneration%20Stream) (Variables|SpawnSettings|GetSpawn%20Amount) (Variables|SpawnSettings|GetRandomization) (Variables|SpawnSettings|GetDefault%20Orbit%20Rotation) (Variables|SpawnSettings|GetDefault%20Rotation) (Variables|SpawnSettings|GetDefault%20Scale) (Variables|SpawnSettings|GetRotate%20relative%20to%20Orbit)))
  (Variables|Default|SetOrbit%20Data _data)
  (for _array_element (Variables|Default|GetActorArray)
    (Components|DestroyComponent _array_element))
  (Utilities|Array|Clear (Variables|Default|GetActorArray))
  (for _array_element_2 (Variables|Default|GetOrbit%20Data)
    (bind (_new_location _new_rotation) (CallFunction|CalculateObjectTransform (.OrbitOffset (Utilities|Struct|BreakStruct_SOMData _array_element_2)) (.OrbitRotation (Utilities|Struct|BreakStruct_SOMData _array_element_2)) (.OrbitRadius (Utilities|Struct|BreakStruct_SOMData _array_element_2)) (.StartAngle (Utilities|Struct|BreakStruct_SOMData _array_element_2)) (.MovementSpeed (Utilities|Struct|BreakStruct_SOMData _array_element_2)) (.RotationSpeed (Utilities|Struct|BreakStruct_SOMData _array_element_2)) (.DefaultRotation (Utilities|Struct|BreakStruct_SOMData _array_element_2)) (.RotaterelativetoOrbit (Utilities|Struct|BreakStruct_SOMData _array_element_2)) 0.0))
    (bind _returnvalue (AddComponent|AddChildActorComponent false (Math|Transform|MakeTransform (- _new_location (Transformation|GetActorLocation)) _new_rotation (.DefaultScale (Utilities|Struct|BreakStruct_SOMData _array_element_2)))))
    (ChildActorComponent|SetChildActorClass _returnvalue (Variables|SpawnSettings|GetActor))
    (Utilities|Array|Add (Variables|Default|GetActorArray) _returnvalue)))

(fn DrawDebugOrbits
  (Components|InstancedStaticMesh|ClearInstances (Variables|Default|GetOverflowOrbitInstancedMeshes))
  (for _index (range 0 (- (Utilities|Array|Length (Variables|Default|GetOrbit%20Data)) 1))
    (CallFunction|AddOrbitPlaneInstance _index (Utilities|Array|Get(acopy) (Variables|Default|GetOrbit%20Data) _index))))