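; Base actor for the Simple Orbit Manager, providing shared logic to move objects along elliptical orbits around itself.
; It snaps to an optional FollowActor at construction and, when enabled, on Tick.
; Helpers compute transforms directly from time, combining tilted orbit, offset, spin and optional orbit-relative facing, but nothing here calls them per frame.
; Other helpers generate orbit data from a seeded random stream and draw debug orbit planes as components or instances.
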(event EventBeginPlay
  (if (not (Variables|Default|GetEnable%20Debug%20Orbits))
    (Components|InstancedStaticMesh|ClearInstances (Variables|Default|GetOverflowOrbitInstancedMeshes))))

(event Collision|EventActorBeginOverlap
  (params (OtherActor :type Actor%20Object%20Reference)))

(event EventTick
  (params (DeltaSeconds :type Float%20%28single-precision%29))
  (if (Variables|Default|GetEnable%20SOM)
    (CallFunction|UpdatePosition)))

(fn ConstructionScript
  (Transformation|SetActorScale3D "1.000000,1.000000,1.000000")
  (Transformation|SetActorRotation "0, 0, 0")
  (CallFunction|UpdatePosition)
  (if (not (Variables|Default|GetShow%20Debug%20Orbits%20in%20Editor))
    (Components|InstancedStaticMesh|ClearInstances (Variables|Default|GetOverflowOrbitInstancedMeshes))))

(fn CalculateOrbitPosition
  (params (Center :type Vector) (Direction :type Rotator) (Angle :type Float%20%28single-precision%29) (WidthX :type Float%20%28single-precision%29) (LengthY :type Float%20%28single-precision%29))
  (return (+ Center (Math|Vector|RotateVector (Math|Vector|MakeVector (* (Math|Trig|Cos(Degrees) Angle) WidthX) (* (Math|Trig|Sin(Degrees) Angle) LengthY) 0.0) Direction))))

(fn UpdateActorPosition
  (params (Actor%20Data :type Struct%20SOM%20Actor%20Data%20Structure) (New%20Time :type Float%20%28single-precision%29))
  (bind (_actor _orbitrotation _orbitradius _orbitoffset _startangle _movementspeed _defaultrotation _rotationspeed _rotaterelativetoorbit) (Utilities|Struct|BreakStruct_SOMActorData Actor%20Data))
  (Utilities|IsValid _actor
    (:Is%20Valid
      (bind (_new_location _new_rotation) (CallFunction|CalculateObjectTransform _orbitoffset _orbitrotation _orbitradius _startangle _movementspeed _rotationspeed _defaultrotation _rotaterelativetoorbit New%20Time))
      (Transformation|SetActorLocationAndRotation _actor _new_location _new_rotation))))

(fn AddOrbitMeshPlane
  (params (Actor%20Data :type Struct%20SOM%20Actor%20Data%20Structure))
  (bind (_actor _orbitrotation _orbitradius _orbitoffset) (Utilities|Struct|BreakStruct_SOMActorData Actor%20Data))
  (bind _returnvalue (Math|Vector|MakeVector 4.0 4.0 4.0))
  (bind (_x _y) (Math|Vector|BreakVector _returnvalue))
  (bind (_x_2 _y_2) (Math|Vector2D|BreakVector2D _orbitradius))
  (bind _returnvalue_2 (AddComponent|AddStaticMeshComponent true (Math|Transform|MakeTransform _orbitoffset _orbitrotation (Math|Vector|MakeVector (* _x (/ _x_2 1e+02)) (* _y (/ _y_2 1e+02)) 1.0))))
  (Transformation|AttachComponentToComponent _returnvalue_2 (Variables|Default|GetOrbitMeshes) "None" "KeepRelative" "KeepRelative" "KeepRelative" false))

(fn CalculateObjectTransform
  (params (Offset :type Vector) (Orbit%20Rotation :type Rotator) (Orbit%20Radius :type Vector%202D%20Structure) (Start%20Angle :type Float%20%28single-precision%29) (Movement%20Speed :type Float%20%28single-precision%29) (Rotation%20Speed :type Rotator) (Default%20Rotation :type Rotator) (Relative%20Rotation :type Boolean) (New%20Time :type Float%20%28single-precision%29))
  (bind (_x _y) (Math|Vector2D|BreakVector2D Orbit%20Radius))
  (bind _returnvalue (* Movement%20Speed New%20Time))
  (bind _returnvalue_2 (+ Start%20Angle _returnvalue))
  (bind _new_location (CallFunction|CalculateOrbitPosition (Transformation|GetActorLocation) Orbit%20Rotation _returnvalue_2 _x _y))
  (return (+ _new_location (Math|Transform|TransformLocation (Math|Transform|MakeTransform "0, 0, 0" Orbit%20Rotation) Offset)) (Math|Transform|TransformRotation (Math|Transform|MakeTransform "0, 0, 0" Orbit%20Rotation) (Math|Transform|TransformRotation (Math|Transform|MakeTransform "0, 0, 0" (Math|Rotator|SelectRotator (Math|Rotator|MakeRotator 0.0 0.0 _returnvalue_2) "0, 0, 0" Relative%20Rotation)) (Math|Transform|TransformRotation (Math|Transform|MakeTransform "0, 0, 0" (* Rotation%20Speed New%20Time)) Default%20Rotation)))))

(fn AddOrbitPlaneInstance
  (params (Index :type Integer) (Orbit%20Data :type Struct%20SOM%20Data%20Structure))
  (bind (_orbitrotation _orbitradius _orbitoffset) (Utilities|Struct|BreakStruct_SOMData Orbit%20Data))
  (bind _returnvalue (Math|Vector|MakeVector 4.0 4.0 4.0))
  (bind (_x _y) (Math|Vector|BreakVector _returnvalue))
  (bind (_x_2 _y_2) (Math|Vector2D|BreakVector2D _orbitradius))
  (Components|InstancedStaticMesh|AddInstance (Variables|Default|GetOverflowOrbitInstancedMeshes) (Math|Transform|MakeTransform (Math|Transform|TransformLocation (Math|Transform|MakeTransform "0, 0, 0" _orbitrotation) _orbitoffset) _orbitrotation (Math|Vector|MakeVector (* _x (/ _x_2 1e+02)) (* _y (/ _y_2 1e+02)) 1.0))))

(fn UpdatePosition
  (bind _follow_actor (Variables|Default|GetFollow%20Actor))
  (Utilities|IsValid _follow_actor
    (:Is%20Valid
      (Transformation|SetActorLocation (Transformation|GetActorLocation _follow_actor) false false))))

(fn ConvertActorDatatoSOMData
  (params (Actor%20Data :type Struct%20SOM%20Actor%20Data%20Structure))
  (bind (_actor _orbitrotation _orbitradius _orbitoffset _startangle _movementspeed _defaultrotation _rotationspeed _rotaterelativetoorbit) (Utilities|Struct|BreakStruct_SOMActorData Actor%20Data))
  (return (Utilities|Struct|MakeStruct_SOMData _orbitrotation _orbitradius _orbitoffset _startangle _movementspeed _defaultrotation _rotationspeed _rotaterelativetoorbit)))

(fn GetRandomVectorinRangefromStream
  (params (Minimum%20Vector :type Vector) (Maximum%20Vector :type Vector) (Random%20Stream :type Random%20Stream%20Structure%20%28by%20ref%29))
  (bind (_x _y _z) (Math|Vector|BreakVector Minimum%20Vector))
  (bind (_x_2 _y_2 _z_2) (Math|Vector|BreakVector Maximum%20Vector))
  (return (Math|Vector|MakeVector (Math|Random|RandomFloatinRangefromStream _x _x_2 Random%20Stream) (Math|Random|RandomFloatinRangefromStream _y _y_2 Random%20Stream) (Math|Random|RandomFloatinRangefromStream _z _z_2 Random%20Stream))))

(fn GetRandomRotatorinRangefromStream
  (params (Minimum%20Rotator :type Rotator) (Maximum%20Rotator :type Rotator) (Random%20Stream :type Random%20Stream%20Structure%20%28by%20ref%29))
  (bind (_roll _pitch _yaw) (Math|Rotator|BreakRotator Minimum%20Rotator))
  (bind (_roll_2 _pitch_2 _yaw_2) (Math|Rotator|BreakRotator Maximum%20Rotator))
  (return (Math|Rotator|MakeRotator (Math|Random|RandomFloatinRangefromStream _roll _roll_2 Random%20Stream) (Math|Random|RandomFloatinRangefromStream _pitch _pitch_2 Random%20Stream) (Math|Random|RandomFloatinRangefromStream _yaw _yaw_2 Random%20Stream))))

(fn GenerateRandomData
  (params (Generation%20Stream :type Random%20Stream%20Structure%20%28by%20ref%29) (Spawn%20Amount :type Integer) (Randomization :type Struct%20SOM%20Randomization%20Structure) (Default%20Orbit%20Rotation :type Rotator) (Default%20Rotation :type Rotator) (Default%20Scale :type Vector) (Rotate%20relative%20to%20Orbit :type Boolean))
  (bind (_minimumorbitrotation _maximumorbitrotation _uniformradius _minimumorbitradius _maximumorbitradius _minimumorbitoffset _maximumorbitoffset _minimumstartangle _maximumstartangle _minimummovementspeed _maximummovementspeed _minimumrotationspeed _maximumrotationspeed _minimumscale _maximumscale) (Utilities|Struct|BreakStruct_SOMRandomization Randomization))
  (bind _x (Math|Vector2D|BreakVector2D _minimumorbitradius))
  (bind _x_2 (Math|Vector2D|BreakVector2D _maximumorbitradius))
  (bind _returnvalue (Math|Random|RandomFloatinRangefromStream _x _x_2 Generation%20Stream))
  (for _index (range 0 (- Spawn%20Amount 1))
    (Utilities|Array|Add (LocalVariables|GetTemp%20Orbit%20Data) (Utilities|Struct|MakeStruct_SOMData (Math|Transform|TransformRotation (Math|Transform|MakeTransform "0, 0, 0" Default%20Orbit%20Rotation) (CallFunction|GetRandomRotatorinRangefromStream _minimumorbitrotation _maximumorbitrotation Generation%20Stream)) (select _uniformradius (Math|Vector2D|MakeVector2D _returnvalue _returnvalue) (Math|Conversions|ToVector2D(Vector) (CallFunction|GetRandomVectorinRangefromStream (Math|Conversions|ToVector(Vector2D) _minimumorbitradius) (Math|Conversions|ToVector(Vector2D) _maximumorbitradius) Generation%20Stream))) (CallFunction|GetRandomVectorinRangefromStream _minimumorbitoffset _maximumorbitoffset Generation%20Stream) (Math|Random|RandomFloatinRangefromStream _minimumstartangle _maximumstartangle Generation%20Stream) (Math|Random|RandomFloatinRangefromStream _minimummovementspeed _maximummovementspeed Generation%20Stream) Default%20Rotation (CallFunction|GetRandomRotatorinRangefromStream _minimumrotationspeed _maximumrotationspeed Generation%20Stream) Rotate%20relative%20to%20Orbit (+ Default%20Scale (CallFunction|GetRandomVectorinRangefromStream _minimumscale _maximumscale Generation%20Stream)))))
  (return (LocalVariables|GetTemp%20Orbit%20Data)))