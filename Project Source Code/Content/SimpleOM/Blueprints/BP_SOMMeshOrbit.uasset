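; Actor that moves instances of a single static mesh along configurable orbits, with optional debug orbit display.
; Construction and BeginPlay rebuild the instances from the OrbitData array and can draw orbit planes as instanced meshes.
; When enabled, Tick recomputes each world transform from time since creation via CalculateObjectTransform.
; Render state is marked dirty only on the last instance update, batching the refresh.
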(event EventBeginPlay
  (|CallParentFunction)
  (CallFunction|InitiateMeshes)
  (if (Variables|Default|GetEnable%20Debug%20Orbits)
    (CallFunction|DrawDebugOrbits)))

(event Collision|EventActorBeginOverlap
  (params (OtherActor :type Actor%20Object%20Reference))
  (|CallParentFunction OtherActor) ; This node is disabled and will not be called.\nDrag off pins to build functionality.
)

(event EventTick
  (params (DeltaSeconds :type Float%20%28single-precision%29))
  (|CallParentFunction DeltaSeconds)
  (if (Variables|Default|GetEnable%20SOM)
    (CallFunction|UpdateAllMeshes (Actor|GetGameTimeSinceCreation))))

(fn ConstructionScript
  (|CallParentFunction)
  (CallFunction|InitiateMeshes)
  (if (Variables|Default|GetShow%20Debug%20Orbits%20in%20Editor)
    (CallFunction|DrawDebugOrbits)))

(fn UpdateAllMeshes
  (params (New%20Time :type Float%20%28single-precision%29))
  (bind _orbit_data (Variables|Default|GetOrbit%20Data))
  (for (_array_element _array_index) _orbit_data
    (bind (_new_location _new_rotation) (CallFunction|CalculateObjectTransform (.OrbitOffset (Utilities|Struct|BreakStruct_SOMData _array_element)) (.OrbitRotation (Utilities|Struct|BreakStruct_SOMData _array_element)) (.OrbitRadius (Utilities|Struct|BreakStruct_SOMData _array_element)) (.StartAngle (Utilities|Struct|BreakStruct_SOMData _array_element)) (.MovementSpeed (Utilities|Struct|BreakStruct_SOMData _array_element)) (.RotationSpeed (Utilities|Struct|BreakStruct_SOMData _array_element)) (.DefaultRotation (Utilities|Struct|BreakStruct_SOMData _array_element)) (.RotaterelativetoOrbit (Utilities|Struct|BreakStruct_SOMData _array_element)) New%20Time))
    (Components|InstancedStaticMesh|UpdateInstanceTransform (Variables|Default|GetMeshes) _array_index (Math|Transform|MakeTransform _new_location _new_rotation (.DefaultScale (Utilities|Struct|BreakStruct_SOMData _array_element))) true (== _array_index (- (Utilities|Array|Length _orbit_data) 1)) false)))

(fn InitiateMeshes
  (Collision|SetCollisionEnabled (Variables|Default|GetMeshes) (Variables|Default|GetCollision%20Type))
  (Components|StaticMesh|SetStaticMesh (Variables|Default|GetMeshes) (Variables|Default|GetStatic%20Mesh))
  (Components|InstancedStaticMesh|ClearInstances (Variables|Default|GetMeshes))
  (for _array_element (Variables|Default|GetOrbit%20Data)
    (bind (_new_location _new_rotation) (CallFunction|CalculateObjectTransform (.OrbitOffset (Utilities|Struct|BreakStruct_SOMData _array_element)) (.OrbitRotation (Utilities|Struct|BreakStruct_SOMData _array_element)) (.OrbitRadius (Utilities|Struct|BreakStruct_SOMData _array_element)) (.StartAngle (Utilities|Struct|BreakStruct_SOMData _array_element)) (.MovementSpeed (Utilities|Struct|BreakStruct_SOMData _array_element)) (.RotationSpeed (Utilities|Struct|BreakStruct_SOMData _array_element)) (.DefaultRotation (Utilities|Struct|BreakStruct_SOMData _array_element)) (.RotaterelativetoOrbit (Utilities|Struct|BreakStruct_SOMData _array_element)) 0.0))
    (Class|InstancedStaticMeshComponent|AddInstanceWorldSpace (Variables|Default|GetMeshes) (Math|Transform|MakeTransform _new_location _new_rotation (.DefaultScale (Utilities|Struct|BreakStruct_SOMData _array_element))))))

(fn DrawDebugOrbits
  (Components|InstancedStaticMesh|ClearInstances (Variables|Default|GetOverflowOrbitInstancedMeshes))
  (for _index (range 0 (- (Utilities|Array|Length (Variables|Default|GetOrbit%20Data)) 1))
    (CallFunction|AddOrbitPlaneInstance _index (Utilities|Array|Get(acopy) (Variables|Default|GetOrbit%20Data) _index))))